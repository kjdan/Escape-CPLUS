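; MainSun animates the day cycle by rotating the Sun actor and refreshing the Sky's sun direction.
; It finds the Creator actor, retrying on Tick while invalid, and advances only while its light value is 1, scaling time by OneDayInMinutes.
; A per-frame countdown, independent of the clock, ends the cycle by resetting state and setting the light value to 0.
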(event `self.ReceiveBeginPlay`
  (bind _outactors (`GameplayStatics.GetAllActorsOfClass` "/Script/MainEngineer.Creator" :!label _label))
  (for _array_element _outactors
    (bind _output_get (set `self.Actor` _array_element))
    (bind _output_get_2 (set `self.OneDay` (* 60.0 (`self.OneDayInMinutes`))))
    (set `self.OneHour` (/ _output_get_2 24.0))))

(event `self.ReceiveTick`
  (params (DeltaSeconds :type "Float (single-precision)"))
  (`/Engine/EditorBlueprintResources/StandardMacros.IsValid` (stale `self.ReceiveBeginPlay` _output_get)
    (:`Is Valid`
      (bind _returnvalue (`Creator.getLightValue` (stale `self.ReceiveBeginPlay` _output_get)))
      (if (== 1 _returnvalue)
        (bind _output_get (set `self.Hour` (+ (`self.Hour`) (/ DeltaSeconds (`self.OneHour`)))))
        (bind _output_get_2 (set `self.Angle` (+ (* (/ _output_get 6.0) 90.0) 90.0)))
        (`self.K2_SetActorRotation` (`self.Sun`) (`KismetMathLibrary.MakeRotator` 0.0 _output_get_2) false)
        (`/Engine/EngineSky/BP_Sky_Sphere.UpdateSunDirection` (`self.Sky`))
        (bind _output_get_3 (set `self.Minus` (- (`self.Minus`) 1.0)))
        (if (== _output_get_3 0.0)
          (bind _output_get_4 (set `self.OneDay` (* 60.0 (`self.OneDayInMinutes`))))
          (set `self.OneHour` (/ _output_get_4 24.0))
          (set `self.Hour` 0.0)
          (set `self.Angle` 0.0)
          (set `self.Minus` 21000.0)
          (`Creator.setLightValue` (stale `self.ReceiveBeginPlay` _output_get) 0))
        (else
          (bind _output_get_5 (set `self.OneDay` (* 60.0 (`self.OneDayInMinutes`))))
          (set `self.OneHour` (/ _output_get_5 24.0))
          (set `self.Hour` 0.0)
          (set `self.Angle` 0.0)
          (set `self.Minus` 21000.0))))
    (:`Is Not Valid`
      (goto _label))))

(fn `UserConstructionScript`)